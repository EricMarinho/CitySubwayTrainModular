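; Interactable suitcase actor that shows a password screen when the player interacts with it nearby.
; SuitcaseTrigger overlaps with BP_FirstPersonCharacter set IsPlayerClose and enable or disable the actor's input for player controller 0.
; While the player is close, the Interact input action creates a new WBP_Password widget on each press and adds it to the viewport.
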(event `EnhancedInput|/Game/FirstPerson/Input/Actions/Interact`
  (params (ActionValue :type Boolean) (ElapsedSeconds :type "Float (double-precision)") (TriggeredSeconds :type "Float (double-precision)") (InputAction :type "InputAction Object Reference" :default "/Game/FirstPerson/Input/Actions/Interact.Interact"))
  (:`Started`
    (if (`self.isPlayerClose`)
      (bind _returnvalue (`|CreateWidget` "/Game/Custom/Blueprints/UI/WBP_Password.WBP_Password_C"))
      (`UserWidget.AddToViewport` _returnvalue 0))))

(event `self.SuitcaseTrigger.OnComponentBeginOverlap`
  (params (OverlappedComponent :type "PrimitiveComponent Object Reference") (OtherActor :type "Actor Object Reference") (OtherComp :type "PrimitiveComponent Object Reference") (OtherBodyIndex :type Integer) (bFromSweep :type Boolean) (SweepResult :type "HitResult Structure (by ref)"))
  (cast `/Game/FirstPerson/Blueprints/BP_FirstPersonCharacter` OtherActor)
  (set `self.isPlayerClose` true)
  (`self.EnableInput` (`GameplayStatics.GetPlayerController` 0)))

(event `self.SuitcaseTrigger.OnComponentEndOverlap`
  (params (OverlappedComponent :type "PrimitiveComponent Object Reference") (OtherActor :type "Actor Object Reference") (OtherComp :type "PrimitiveComponent Object Reference") (OtherBodyIndex :type Integer))
  (cast `/Game/FirstPerson/Blueprints/BP_FirstPersonCharacter` OtherActor)
  (set `self.isPlayerClose` false)
  (`self.DisableInput` (`GameplayStatics.GetPlayerController` 0)))

(fn `UserConstructionScript`)